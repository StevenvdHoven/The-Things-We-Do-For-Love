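; Player controller that routes Enhanced Input actions to the possessed BP_Player.
; It adds the action mapping context on BeginPlay, then forwards move, dodge, look, sprint, attack and lock-toggle input to matching functions on the pawn.
; Move and dodge get normalized directions built from the camera's forward and right vectors, making them camera-relative, and attack gets the camera forward vector.
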(event Input|EnhancedActionEvents|EnhancedInputActionIA_Move
  (params (ActionValue :type Vector%202D%20Structure) (ElapsedSeconds :type Float%20%28double-precision%29) (TriggeredSeconds :type Float%20%28double-precision%29) (InputAction :type Input%20Action%20Object%20Reference :default "/Game/Game/Player/Input/Actions/IA_Move.IA_Move"))
  (bind (_x _y) (Math|Vector2D|BreakVector2D ActionValue))
  (bind _returnvalue (Game|GetPlayerCameraManager 0))
  (bind _returnvalue_2 (Camera|GetCameraRotation _returnvalue))
  (:Triggered
    (bind _asbp_player (Utilities|Casting|CastToBP_Player (Pawn|GetControlledPawn)))
    (Class|CombatCharacter|Move _asbp_player (Math|Vector|Normalize (+ (* _x (Math|Vector|GetRightVector _returnvalue_2)) (* _y (Math|Vector|GetForwardVector _returnvalue_2)))) ActionValue)))

(event Input|EnhancedActionEvents|EnhancedInputActionIA_Look
  (params (ActionValue :type Vector%202D%20Structure) (ElapsedSeconds :type Float%20%28double-precision%29) (TriggeredSeconds :type Float%20%28double-precision%29) (InputAction :type Input%20Action%20Object%20Reference :default "/Game/Game/Player/Input/Actions/IA_Look.IA_Look"))
  (bind _asbp_player (Utilities|Casting|CastToBP_Player (Pawn|GetControlledPawn)))
  (Class|CombatCharacter|Look _asbp_player ActionValue))

(event Input|EnhancedActionEvents|EnhancedInputActionIA_Sprint
  (params (ActionValue :type Boolean) (ElapsedSeconds :type Float%20%28double-precision%29) (TriggeredSeconds :type Float%20%28double-precision%29) (InputAction :type Input%20Action%20Object%20Reference :default "/Game/Game/Player/Input/Actions/IA_Sprint.IA_Sprint"))
  (bind _asbp_player (Utilities|Casting|CastToBP_Player (Pawn|GetControlledPawn)))
  (Class|CombatCharacter|Sprint _asbp_player ActionValue))

(event Input|EnhancedActionEvents|EnhancedInputActionIA_Attack
  (params (ActionValue :type Boolean) (ElapsedSeconds :type Float%20%28double-precision%29) (TriggeredSeconds :type Float%20%28double-precision%29) (InputAction :type Input%20Action%20Object%20Reference :default "/Game/Game/Player/Input/Actions/IA_Attack.IA_Attack"))
  (bind _asbp_player (Utilities|Casting|CastToBP_Player (Pawn|GetControlledPawn)))
  (Class|CombatCharacter|Attack _asbp_player (Math|Vector|GetForwardVector (Camera|GetCameraRotation (Game|GetPlayerCameraManager 0)))))

(event Input|EnhancedActionEvents|EnhancedInputActionIA_Dodge
  (params (ActionValue :type Boolean) (ElapsedSeconds :type Float%20%28double-precision%29) (TriggeredSeconds :type Float%20%28double-precision%29) (InputAction :type Input%20Action%20Object%20Reference :default "/Game/Game/Player/Input/Actions/IA_Dodge.IA_Dodge"))
  (bind _returnvalue (Game|GetPlayerCameraManager 0))
  (bind _returnvalue_2 (Camera|GetCameraRotation _returnvalue))
  (bind _asbp_player (Utilities|Casting|CastToBP_Player (Pawn|GetControlledPawn)))
  (Class|CombatCharacter|Dodge _asbp_player (Math|Vector|Normalize (+ (* (Math|Vector|GetForwardVector _returnvalue_2) (.Y (Math|Vector2D|BreakVector2D (stale Input|EnhancedActionEvents|EnhancedInputActionIA_Move ActionValue)))) (* (.X (Math|Vector2D|BreakVector2D (stale Input|EnhancedActionEvents|EnhancedInputActionIA_Move ActionValue))) (Math|Vector|GetRightVector _returnvalue_2))))))

(event Input|EnhancedActionEvents|EnhancedInputActionIA_Lock
  (params (ActionValue :type Boolean) (ElapsedSeconds :type Float%20%28double-precision%29) (TriggeredSeconds :type Float%20%28double-precision%29) (InputAction :type Input%20Action%20Object%20Reference :default "/Game/Game/Player/Input/Actions/IA_Lock.IA_Lock"))
  (bind _asbp_player (Utilities|Casting|CastToBP_Player (Pawn|GetControlledPawn)))
  (Class|CombatCharacter|ToggleLock _asbp_player))

(event EventBeginPlay
  (Input|AddMappingContext (PlayerController|LocalPlayerSubsystems|GetEnhancedInputLocalPlayerSubsystem) "/Game/Game/Player/Input/IMC_ActionMap.IMC_ActionMap" 0 "(bIgnoreAllPressedKeysUntilRelease=True,bForceImmediately=False,bNotifyUserSettings=False)"))

(fn ConstructionScript)