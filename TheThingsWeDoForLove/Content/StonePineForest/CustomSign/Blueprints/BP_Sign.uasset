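; BP_Sign is a customizable sign actor that builds its shape, icon, text and colors in the Construction Script.
; The sign type picks the mesh from the DT_Signs data table.
; A canvas render target update draws the icon texture and text.
; That same update creates a dynamic material, feeding it the render target, a per-type RGB mask, detail UV scale and color parameters.
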(event EventBeginPlay)

(event Collision|EventActorBeginOverlap
  (params (OtherActor :type Actor%20Object%20Reference)))

(event EventTick
  (params (DeltaSeconds :type Float%20%28single-precision%29)))

(fn ConstructionScript
  (Utilities|FlowControl|Sequence
    (:then_0
      (switch Utilities|FlowControl|Switch|SwitchonE_SignTypes (Variables|SignProperties|GetSign_Type)
        (:NewEnumerator0
          (bind _returnvalue (Utilities|GetDataTableRow "/Game/StonePineForest/CustomSign/Blueprints/DT_Signs.DT_Signs" "Circle")
            (:then
              (Components|StaticMesh|SetStaticMesh (Variables|Default|GetSM_SignMesh) (.Mesh (Utilities|Struct|BreakStruct_Signs _returnvalue))))))
        (:NewEnumerator1
          (bind _returnvalue_2 (Utilities|GetDataTableRow "/Game/StonePineForest/CustomSign/Blueprints/DT_Signs.DT_Signs" "Rectangle")
            (:then
              (Components|StaticMesh|SetStaticMesh (Variables|Default|GetSM_SignMesh) (.Mesh (Utilities|Struct|BreakStruct_Signs _returnvalue_2))))))
        (:NewEnumerator2
          (bind _returnvalue_3 (Utilities|GetDataTableRow "/Game/StonePineForest/CustomSign/Blueprints/DT_Signs.DT_Signs" "Direction")
            (:then
              (Components|StaticMesh|SetStaticMesh (Variables|Default|GetSM_SignMesh) (.Mesh (Utilities|Struct|BreakStruct_Signs _returnvalue_3))))))
        (:NewEnumerator3
          (bind _returnvalue_4 (Utilities|GetDataTableRow "/Game/StonePineForest/CustomSign/Blueprints/DT_Signs.DT_Signs" "Square")
            (:then
              (Components|StaticMesh|SetStaticMesh (Variables|Default|GetSM_SignMesh) (.Mesh (Utilities|Struct|BreakStruct_Signs _returnvalue_4))))))
        (:NewEnumerator5
          (bind _returnvalue_5 (Utilities|GetDataTableRow "/Game/StonePineForest/CustomSign/Blueprints/DT_Signs.DT_Signs" "Triangle")
            (:then
              (Components|StaticMesh|SetStaticMesh (Variables|Default|GetSM_SignMesh) (.Mesh (Utilities|Struct|BreakStruct_Signs _returnvalue_5))))))))
    (:then_1
      (bind _returnvalue_6 (CanvasRenderTarget2D|CreateCanvasRenderTarget2D "/Script/Engine.CanvasRenderTarget2D" 2048 2048))
      (bind _output_get (Variables|Default|SetRenderTarget _returnvalue_6))
      (EventDispatchers|BindEventtoOnCanvasRenderTargetUpdate _output_get (EventDispatchers|CreateEvent :!event BPSignAutoGenFunc)))
    (:then_2
      (Class|CanvasRenderTarget2D|UpdateResource (Variables|Default|GetRenderTarget)))))

(fn BPSignAutoGenFunc
  (params (Canvas :type Canvas%20Object%20Reference) (Width :type Integer) (Height :type Integer))
  (bind _sm_signmesh (Variables|Default|GetSM_SignMesh))
  ;[1 1 1] Draws icon texture and text on render target
  (Canvas|DrawTexture :self Canvas :RenderTexture (Variables|IconProperties|GetIconTexture) :ScreenPosition (Math|Vector2D|MakeVector2D (Variables|IconProperties|GetIconPositionX) (Variables|IconProperties|GetIconPositionY)) :ScreenSize (/ (Math|Vector2D|MakeVector2D (Math|Conversions|ToFloat(Integer) Width) (Math|Conversions|ToFloat(Integer) Height)) (Variables|IconProperties|GetIconSize)) :CoordinateSize "(X=1.000000,Y=1.000000)" :RenderColor "(R=1.000000,G=1.000000,B=1.000000,A=0.000000)" :BlendMode "BLEND_Masked" :PivotPoint "(X=0.500000,Y=0.500000)")
  (HUD|DrawText Canvas (Variables|TextProperties|GetTextFont) (Variables|TextProperties|GetTextInput) "(X=15.000000,Y=15.000000)" "(X=5.000000,Y=5.000000)" "(R=1.000000,G=1.000000,B=1.000000,A=1.000000)" 0.0 "(R=0.000000,G=0.000000,B=0.000000,A=1.000000)" "(X=1.000000,Y=1.000000)" false false false "(R=0.000000,G=0.000000,B=0.000000,A=1.000000)")
  ;[0 0 1] Creates a new dynamic material instance and sets it to Sign Mesh
  (bind _returnvalue (Rendering|Material|CreateDynamicMaterialInstance _sm_signmesh 0 "/Game/StonePineForest/CustomSign/Materials/MI_OnlyForBP.MI_OnlyForBP" "None" :!class /Script/Engine.PrimitiveComponent))
  (Rendering|Material|SetMaterial _sm_signmesh 0 _returnvalue)
  ;[1 1 0] Switches Mask Texture and UV Coordinate parameters based on Sign Type. Background elements use RGB Mask and UVCoords scale sign details that come from normal, roughness, specular and ambient occ textures.
  (switch Utilities|FlowControl|Switch|SwitchonE_SignTypes (Variables|SignProperties|GetSign_Type)
    (:NewEnumerator0
      ;[1 1 1] Feeds set settings to material
      (Utilities|DynamicMatValues _returnvalue "/Game/StonePineForest/CustomSign/Textures/T_Circle_Mask.T_Circle_Mask" 1.0))
    (:NewEnumerator1
      (Utilities|DynamicMatValues _returnvalue "/Game/StonePineForest/CustomSign/Textures/T_Rectangle_Mask.T_Rectangle_Mask" 1.3))
    (:NewEnumerator2
      (Utilities|DynamicMatValues _returnvalue "/Game/StonePineForest/CustomSign/Textures/T_DirectionRec_Mask.T_DirectionRec_Mask" 2.0))
    (:NewEnumerator3
      (Utilities|DynamicMatValues _returnvalue "/Game/StonePineForest/CustomSign/Textures/T_Square_Mask.T_Square_Mask" 0.0))
    (:NewEnumerator5
      (Utilities|DynamicMatValues _returnvalue "/Game/StonePineForest/CustomSign/Textures/T_Triangle_Mask.T_Triangle_Mask" 1.0))))